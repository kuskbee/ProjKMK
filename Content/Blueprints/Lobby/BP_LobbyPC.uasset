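; BP_LobbyPC is a lobby player controller Blueprint that moves the client onto a dedicated game server when the match starts.
; On BeginPlay it binds a handler to the LoginClientSubsystem's start-game delegate.
; OnStartGame joins the received IP and port into an address string and opens it as a level, connecting the client to that server.
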(event `self.ReceiveBeginPlay`
  (add `LoginClientSubsystem.OnStartGameDelegate` (subsystem `LoginClientSubsystem`) (`|CreateDelegate` :!event `OnStartGame`)))

(fn `OnStartGame`
  (params (DediIp :type String) (DediPort :type Integer))
  (locals (ServerAddress :type String))
  (bind _output_get (set `local.ServerAddress` (`KismetStringLibrary.Concat_StrStr` DediIp ":" (`KismetStringLibrary.Conv_IntToString` DediPort))))
  (`GameplayStatics.OpenLevel` (`KismetStringLibrary.Conv_StringToName` (`local.ServerAddress`))))

(fn `UserConstructionScript`)
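; Game instance Blueprint for an entry test that tracks lobby players and their ready states.
; On Init it binds to LoginClientSubsystem delegates for player list, join/leave and state changes, retrying on a short timer until the subsystem is valid.
; The handlers update a PlayerList map keyed by UserId, then fire dispatchers for list, count, join/leave and readiness changes, including a separate one for the local player's ready state.
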(event `self.ReceiveInit`
  (`self.BindLoginClientEvent`))

(fn `BindLoginClientEvent`
  (bind _returnvalue (subsystem `LoginClientSubsystem`))
  (`/Engine/EditorBlueprintResources/StandardMacros.IsValid` _returnvalue
    (:`Is Valid`
      (add `LoginClientSubsystem.OnPlayerListResponseDelegate` _returnvalue (`|CreateDelegate` :!event `OnResponsePlayerList`))
      (add `LoginClientSubsystem.OnPlayerInOutLobbyDelegate` _returnvalue (`|CreateDelegate` :!event `OnPlayerInOutLobby`))
      (add `LoginClientSubsystem.OnPlayerChangeStateDelegate` _returnvalue (`|CreateDelegate` :!event `OnPlayerChangeState`)))
    (:`Is Not Valid`
      (`KismetSystemLibrary.K2_SetTimer` null "BindLoginClientEvent" 0.01))))

(fn `OnPlayerChangeState`
  (params (UserId :type String) (CurrentState :type "EEntryState Enum" :default "EPS_Lobby"))
  (bind (_value _returnvalue) (`BlueprintMapLibrary.Map_Find` (`self.PlayerList`) UserId))
  (bind (_userid _nickname) (break `PlayerInfo` _value))
  (if _returnvalue
    (`|ExecutionSequence`
      (:`then_0`
        ; 찾으면 새 CurrentState 값으로 갱신
        (`BlueprintMapLibrary.Map_Add` (`self.PlayerList`) (`local.UserId`) (make `PlayerInfo` _userid _nickname (`local.CurrentState`)))
        (`self.EventDispatcher_PlayerReady` _nickname (`|EnumEquality` "EPS_Ready" (`local.CurrentState`))))
      (:`then_1`
        (if (`KismetStringLibrary.EqualEqual_StrStr` _nickname (`self.Nickname`))
          (`self.EventDispatcher_ChangeMyReadyState` (`|EnumEquality` "EPS_Ready" (`local.CurrentState`))))))))

(fn `OnPlayerInOutLobby`
  (params (PlayerInfo :type "PlayerInfo Structure") (bIsJoin :type Boolean))
  (bind _playerinfo (`local.PlayerInfo`))
  (bind (_userid _nickname) (break `PlayerInfo` _playerinfo))
  (`|ExecutionSequence`
    (:`then_0`
      (if bIsJoin
        (`BlueprintMapLibrary.Map_Add` (`self.PlayerList`) _userid _playerinfo)
        (`self.EventDispatcher_AddPlayerOne` _nickname)
        (else
          (`BlueprintMapLibrary.Map_Remove` (`self.PlayerList`) _userid)
          (`self.EventDispatcher_RemovePlayerOne` _nickname))))
    (:`then_1`
      (`self.EventDispatcher_ChangePlayerCnt` (`BlueprintMapLibrary.Map_Length` (`self.PlayerList`))))))

(fn `OnResponsePlayerList`
  (params (PlayerInfos :type "Array of PlayerInfo Structure (by ref)"))
  (for _array_element PlayerInfos
    (`BlueprintMapLibrary.Map_Add` (`self.PlayerList`) (`.UserId` (break `PlayerInfo` _array_element)) _array_element))
  (`self.EventDispatcher_PlayerList`)
  (`self.EventDispatcher_ChangePlayerCnt` (`BlueprintMapLibrary.Map_Length` (`self.PlayerList`))))
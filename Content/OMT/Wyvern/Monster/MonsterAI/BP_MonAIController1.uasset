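; AI controller for the Wyvern monster that runs the BT_MonAI_Test behavior tree and starts chases.
; When perception updates on an Echo character, it sets TargetActor and the Chase state in the Blackboard and mirrors the state on the Wyvern, unless already in Battle.
; In the third phase it also shows the HUD health bar bound to the Wyvern.
; A Blackboard-polling state-change dispatcher exists, but its timer is never run.
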(event `self.ReceiveBeginPlay`
  (`self.RunBehaviorTree` "/MonsterPlugin/Wyvern/Monster/MonsterAI/BT_MonAI_Test.BT_MonAI_Test"))

(event `self.AIPerception.OnTargetPerceptionUpdated`
  (params (Actor :type "Actor Object Reference") (Stimulus :type "AIStimulus Structure"))
  (bind _asbp_echo_character (cast `/EchoCharacterPlugin/Blueprints/Character/Echo/BP_EchoCharacter` Actor)) ; Echo일 때만 Chase하도록 처리
  (`self.ChasePlayer` _asbp_echo_character))

(fn `ChasePlayer`
  (params (Actor :type "Actor Object Reference"))
  (bind _returnvalue (enumliteral `/MonsterPlugin/Wyvern/Monster/MonsterAI/EN_MonAIState` "NewEnumerator2"))
  (bind _asbp_first_phase_wyvern (cast `/MonsterPlugin/Wyvern/Monster/Blueprints/BP_FirstPhaseWyvern` (`self.K2_GetPawn`)))
  ; AIPerception에 감지 시 Blackboard Enum 변경(State 전환)
  (if (`|EnumInequality` (`/MonsterPlugin/Wyvern/Monster/Blueprints/BP_FirstPhaseWyvern.MonAIState` _asbp_first_phase_wyvern) "NewEnumerator3")
    (`|ExecutionSequence`
      (:`then_0`
        (`BlackboardComponent.SetValueAsObject` (`AIBlueprintHelperLibrary.GetBlackboard` null) "TargetActor" Actor)
        (`BlackboardComponent.SetValueAsEnum` (`AIBlueprintHelperLibrary.GetBlackboard` null) "MonAIState" _returnvalue))
      (:`then_1`
        ; Wyvern의 Enum 변경(State 동기화)
        (set `/MonsterPlugin/Wyvern/Monster/Blueprints/BP_FirstPhaseWyvern.MonAIState` _returnvalue _asbp_first_phase_wyvern))
      (:`then_2`
        ; (ThirdPhase 일 때만) HUD - Monster HPbar
        (if (`|EnumEquality` (`/MonsterPlugin/Wyvern/Monster/Blueprints/BP_FirstPhaseWyvern.Phase` _asbp_first_phase_wyvern) "NewEnumerator2")
          (`self.ShowMonsterHealthBar`))))))

(fn `ShowMonsterHealthBar`
  (bind _asbp_hud (cast `/UiPlugin/CRPlugIn/Content/BluePrints/BP_Hud` (`PlayerController.GetHUD` (`GameplayStatics.GetPlayerController` 0))))
  (if (not (`/UiPlugin/CRPlugIn/Content/BluePrints/BP_Hud.IsShowHealthBar` _asbp_hud))
    (`/UiPlugin/CRPlugIn/Content/BluePrints/BP_Hud.ShowMonsterHealthBar` _asbp_hud)
    (bind _asbp_first_phase_wyvern (cast `/MonsterPlugin/Wyvern/Monster/Blueprints/BP_FirstPhaseWyvern` (`self.K2_GetPawn`)))
    (`/UiPlugin/CRPlugIn/Content/BluePrints/BP_Hud.BindWyvernEvent` _asbp_hud _asbp_first_phase_wyvern)))

(fn `UpdateMonState`
  (bind _returnvalue (cast `/MonsterPlugin/Wyvern/Monster/MonsterAI/EN_MonAIState` (`BlackboardComponent.GetValueAsEnum` (`AIBlueprintHelperLibrary.GetBlackboard` null) "MonAIState")))
  (if (not (`|EnumEquality` _returnvalue (`self.MonAIState`)))
    (bind _output_get (set `self.MonAIState` _returnvalue))
    (`self.EventDispatcher_ChangeMonAIState` _output_get)))

(fn `UserConstructionScript`)